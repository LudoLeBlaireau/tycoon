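; BP_generateur is an actor Blueprint that opens the W_ressources widget on screen when play begins.
; BeginPlay creates and stores the widget, adds it to the viewport, then switches the first player controller to UI-only input with a visible mouse cursor.
; A duplicate chain for a W_test widget is left unconnected and never runs, and the construction script is empty.
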(event EventBeginPlay
  (bind _returnvalue (Game|GetPlayerController 0))
  (bind _returnvalue_2 (UserInterface|CreateWidget "/Game/W_ressources.W_ressources_C"))
  (bind _output_get (Variables|Default|Setwidget _returnvalue_2))
  (UserInterface|Viewport|AddtoViewport _output_get 0)
  (Input|SetInputModeUIOnly _returnvalue 0 "DoNotLock" false)
  (Variables|/Script/Engine.PlayerController|SetbShowMouseCursor _returnvalue true))

(fn ConstructionScript)